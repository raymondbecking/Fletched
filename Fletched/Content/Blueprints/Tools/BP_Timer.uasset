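; BP_Timer is a stopwatch actor that times the player through three overlap volumes: Start, Stop and Reset.
; Entering Start runs the timer and adds a WBP_Timer widget to the viewport, and entering Stop halts counting.
; Leaving Reset after the timer is created removes the widgets and zeroes the time.
; Tick counts Seconds and Minutes through a one-second Delay rather than a timer handle.
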(event OnComponentBeginOverlap(Start)
  (params (OverlappedComponent :type Primitive%20Component%20Object%20Reference) (OtherActor :type Actor%20Object%20Reference) (OtherComp :type Primitive%20Component%20Object%20Reference) (OtherBodyIndex :type Integer) (bFromSweep :type Boolean) (SweepResult :type Hit%20Result%20Structure%20%28by%20ref%29))
  ;[1 1 1] Start Timer
  (Utilities|Casting|CastToPlayerCharacter OtherActor)
  (Utilities|FlowControl|Sequence
    (:then_0
      (Variables|Default|SetbTimerCreated true)
      (Variables|Default|SetbTimerIsRunning true))
    (:then_1
      (bind _returnvalue (UserInterface|CreateWidget "/Game/UI/HUD/WBP_Timer.WBP_Timer_C"))
      (UserInterface|Viewport|AddtoViewport _returnvalue 0))))

(event OnComponentBeginOverlap(Stop)
  (params (OverlappedComponent :type Primitive%20Component%20Object%20Reference) (OtherActor :type Actor%20Object%20Reference) (OtherComp :type Primitive%20Component%20Object%20Reference) (OtherBodyIndex :type Integer) (bFromSweep :type Boolean) (SweepResult :type Hit%20Result%20Structure%20%28by%20ref%29))
  ;[1 1 1] Stop Timer
  (Utilities|Casting|CastToPlayerCharacter OtherActor)
  (Variables|Default|SetbTimerIsRunning false))

(event OnComponentEndOverlap(Reset)
  (params (OverlappedComponent :type Primitive%20Component%20Object%20Reference) (OtherActor :type Actor%20Object%20Reference) (OtherComp :type Primitive%20Component%20Object%20Reference) (OtherBodyIndex :type Integer))
  ;[1 1 1] Remove Timer
  (Utilities|Casting|CastToPlayerCharacter OtherActor)
  (if (Variables|Default|GetbTimerCreated)
    (Utilities|FlowControl|Sequence
      (:then_0
        (bind _foundwidgets (Widget|GetAllWidgetsOfClass "/Game/UI/HUD/WBP_Timer.WBP_Timer_C" true))
        (Widget|RemovefromParent _foundwidgets)
        (Variables|Default|SetbTimerIsRunning false)
        (Variables|Default|SetbTimerCreated false))
      (:then_1
        (Variables|Default|SetSeconds 0)
        (Variables|Default|SetMinutes 0)))))

(event EventTick
  (params (DeltaSeconds :type Float%20%28single-precision%29))
  ;[1 1 1] Timer logic
  (if (Variables|Default|GetbTimerIsRunning)
    (Utilities|FlowControl|Sequence
      (:then_1
        (Utilities|FlowControl|Delay 1.0)
        (bind _result (Math|Integer|IncrementInt (Variables|Default|GetSeconds))
          (:%20%20
            (bind _output_get (Variables|Default|SetSeconds _result))
            (if (> _output_get 59)
              (Variables|Default|SetSeconds 0)
              (bind _result_2 (Math|Integer|IncrementInt (Variables|Default|GetMinutes))
                (:%20%20
                  (Variables|Default|SetMinutes _result_2))))))))))

(fn ConstructionScript)